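; Main menu controller that opens the game's front-end menu and routes player input to it.
; On BeginPlay it applies the widget menu input mapping context, fades the camera, then creates the MainMenu_W widget with saved settings and a visible cursor.
; The first key press advances the menu state once through a DoOnce.
; Enhanced Input select, navigate and back actions forward directly to the widget.
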(event Input|EnhancedActionEvents|EnhancedInputActionSelect_IA
  (params (ActionValue :type Boolean) (ElapsedSeconds :type Float%20%28double-precision%29) (TriggeredSeconds :type Float%20%28double-precision%29) (InputAction :type Input%20Action%20Object%20Reference :default "/Game/StoryFramework/Core/Blueprints/ExampleInput/Actions/Shared/Select_IA.Select_IA"))
  (:Started
    (Default|SelectHoveredButton (Variables|Default|GetMainMenuWidgetRef))))

(event Input|EnhancedActionEvents|EnhancedInputActionBack_IA
  (params (ActionValue :type Boolean) (ElapsedSeconds :type Float%20%28double-precision%29) (TriggeredSeconds :type Float%20%28double-precision%29) (InputAction :type Input%20Action%20Object%20Reference :default "/Game/StoryFramework/Core/Blueprints/ExampleInput/Actions/Shared/Back_IA.Back_IA"))
  (:Started
    (Default|BackPage (Variables|Default|GetMainMenuWidgetRef))))

(event Input|EnhancedActionEvents|EnhancedInputActionNavigate_IA
  (params (ActionValue :type Vector%202D%20Structure) (ElapsedSeconds :type Float%20%28double-precision%29) (TriggeredSeconds :type Float%20%28double-precision%29) (InputAction :type Input%20Action%20Object%20Reference :default "/Game/StoryFramework/Core/Blueprints/ExampleInput/Actions/Shared/Navigate_IA.Navigate_IA"))
  (:Started
    (Default|Navigate (Variables|Default|GetMainMenuWidgetRef) ActionValue)))

(event EventBeginPlay
  (CallFunction|UpdateInputMappingContext "/Game/StoryFramework/Menus/Input/WidgetMenu_IMC.WidgetMenu_IMC" true)
  (CallFunction|WidgetFadeCamera -1 1e+01)
  (bind _returnvalue (UserInterface|CreateWidget "/Game/StoryFramework/Menus/UserInterface/MainMenu_W.MainMenu_W_C"))
  (bind _output_get (Variables|Default|SetMainMenuWidgetRef _returnvalue))
  (Widget|SetFocus _output_get)
  (Default|LoadSettings _output_get)
  (UserInterface|Viewport|AddtoViewport _output_get 0)
  (Variables|/Script/Engine.PlayerController|SetbShowMouseCursor (Game|GetPlayerController 0) true))

(event Input|KeyboardEvents|AnyKey
  (params (Key :type Key%20Structure))
  (:Pressed
    (Utilities|FlowControl|DoOnce false
      (:Completed
        (Default|UpdateMenuStatebyIndex (Variables|Default|GetMainMenuWidgetRef) 1)))))

(fn ConstructionScript)