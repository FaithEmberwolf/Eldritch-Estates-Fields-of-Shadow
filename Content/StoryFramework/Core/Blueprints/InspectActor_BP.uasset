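; InspectActor_BP is a 3D item inspection actor that shows a given mesh for the player to rotate.
; On creation it sets the mesh, offset and starting yaw, then places a SceneCaptureComponent2D at the supplied distance, restricted to rendering only that mesh.
; RotateComponent turns 2D input into pitch and yaw on the mesh, doubling the speed when a gamepad is in use.
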(event Custom|OnCreated
  (params (ItemMesh :type Static%20Mesh%20Object%20Reference) (MeshOffset :type Vector) (ActorDistanceFromCamera :type Float%20%28double-precision%29))
  ;[0.04314 0.04314 0.05098] Systems (Root)
  (|OnCreatedLogic ItemMesh MeshOffset ActorDistanceFromCamera))

(event Custom|RotateComponent
  (params (Direction :type Vector%202D%20Structure))
  ;[0.04314 0.04314 0.05098] Systems (Root)
  (|RotateComponentLogic Direction))

(fn ConstructionScript)