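; Base Story Framework Blueprint for interactable objects, with empty hooks for interaction and for loading from a SaveGame data string.
; An InteractionData variable supplies the static mesh, and setting it refreshes the interaction widget component and cosmetics.
; The construction script and the data setter both apply the cosmetics and resize the collision sphere to a custom radius.
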(event Custom|UpdateCosmetics
  (|UpdateCosmeticsLogic))

(event Custom|LoadFromDataString
  (params (DataString :type String)))

(event EventInteractwith
  (params (DataString :type String)))

(event EventUpdateInteractionData
  (params (InteractionData :type Interactable%20Data%20S%20Structure))
  (|SetInteractionData InteractionData))

(fn ConstructionScript
  (CallFunction|UpdateCosmetics)
  (Components|Sphere|SetSphereRadius (Variables|Default|GetSphere) (Variables|Default|GetCustomCollisionRadius) true))

(fn GetInteractionData
  (return (Variables|Default|GetInteractionData)))