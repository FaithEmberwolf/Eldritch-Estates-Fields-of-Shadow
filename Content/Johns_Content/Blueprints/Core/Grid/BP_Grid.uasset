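; BP_Grid spawns a square, hexagon or triangle grid of BP_Plot tile actors from its own location on BeginPlay.
; SpawnGrid clears old tiles, snaps the center, derives a bottom-left origin, then places tiles using per-shape spacing and mesh size from DT_GridShapeData.
; Hexagons stagger by stepping alternate Y indices over a doubled range, while other shapes use the X count on both axes.
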(event EventBeginPlay
  (CallFunction|SpawnGrid (Transformation|GetActorLocation) (Variables|Default|GetGridTileSize) (Variables|Default|GetGridShape) (Variables|Default|GetGridTileCount)))

(fn ConstructionScript)

(fn SpawnGrid
  (params (CenterLocation :type Vector) (TileSize :type Vector) (Shape :type E_GridShape%20Enum :default "NewEnumerator0") (TileCount :type Int%20Point%20Structure))
  (Variables|Default|SetGridCenterLocation CenterLocation)
  (Variables|Default|SetGridTileSize TileSize)
  (Variables|Default|SetGridShape Shape)
  (Variables|Default|SetGridTileCount TileCount)
  (CallFunction|DestroyGrid)
  (bind (_center _bottomleft) (CallFunction|CalculateBottomLeftandCenter))
  (Variables|Default|SetGridCenterLocation _center)
  (Variables|Default|SetGridBottomLeftCornerLocation _bottomleft)
  (for _index (range 0 (- (.x (Variables|Default|GetGridTileCount)) 1))
    (LocalVariables|Setx _index)
    (if (Utilities|Enum|NotEqual(Enum) (Variables|Default|GetGridShape) "NewEnumerator2")
      (for _index_2 (range 0 (- (.x (Variables|Default|GetGridTileCount)) 1))
        (LocalVariables|Sety _index_2)
        (LocalVariables|SetIndex (Utilities|Struct|MakeIntPoint (LocalVariables|Getx) (LocalVariables|Gety)))
        (bind _output_get (LocalVariables|SetTileTransform (Math|Transform|MakeTransform (+ (CallFunction|GetTileLocationfromGridIndex (LocalVariables|GetIndex)) "0.000000,0.000000,2.000000") (CallFunction|GetTileRotationfromGridIndex (LocalVariables|GetIndex)) (/ (Variables|Default|GetGridTileSize) (.MeshSize (Utilities|Struct|BreakS_GridShapeData (CallFunction|GetCurrentShapeData)))))))
        (bind _returnvalue (Game|SpawnActorfromClass "/Game/Johns_Content/Blueprints/Core/Plots/BP_Plot.BP_Plot_C" _output_get "Undefined" "MultiplyWithRoot" 0 0))
        (Utilities|Array|Add (Variables|Default|GetTiles) _returnvalue))
      (else
        (for _index_3 (range (Math|Integer|SelectInt 0 1 (CallFunction|IsIntEven (LocalVariables|Getx))) (- (* (.y (Variables|Default|GetGridTileCount)) 2) 1))
          (LocalVariables|Sety _index_3)
          (Utilities|FlowControl|Sequence
            (:then_0
              (LocalVariables|SetIndex (Utilities|Struct|MakeIntPoint (LocalVariables|Getx) (LocalVariables|Gety)))
              (bind _output_get_2 (LocalVariables|SetTileTransform (Math|Transform|MakeTransform (+ (CallFunction|GetTileLocationfromGridIndex (LocalVariables|GetIndex)) "0.000000,0.000000,2.000000") (CallFunction|GetTileRotationfromGridIndex (LocalVariables|GetIndex)) (/ (Variables|Default|GetGridTileSize) (.MeshSize (Utilities|Struct|BreakS_GridShapeData (CallFunction|GetCurrentShapeData)))))))
              (bind _returnvalue_2 (Game|SpawnActorfromClass "/Game/Johns_Content/Blueprints/Core/Plots/BP_Plot.BP_Plot_C" _output_get_2 "Undefined" "MultiplyWithRoot" 0 0))
              (Utilities|Array|Add (Variables|Default|GetTiles) _returnvalue_2))
            (:then_1
              (Math|Integer|IncrementInt _index_3))))))))

(fn GetCurrentShapeData
  (bind _gridshape (Variables|Default|GetGridShape))
  (bind _returnvalue (Utilities|String|EnumtoString _gridshape))
  (bind _returnvalue_2 (Utilities|GetDataTableRow "/Game/Johns_Content/Variables/DataTables/DT_GridShapeData.DT_GridShapeData" (Utilities|String|StringToName _returnvalue))
    (:then
      _)
    (:RowNotFound
      (Development|PrintString (Utilities|String|Append "Error - Row Not Found - " _returnvalue) true true "(R=1.000000,G=0.000000,B=0.010850,A=1.000000)" 5.0 "GridShapeData")))
  (return _returnvalue_2))

(fn DestroyGrid
  (for _array_element (Variables|Default|GetTiles)
    (Actor|DestroyActor _array_element))
  (Utilities|Array|Clear (Variables|Default|GetTiles)))

(fn CalculateBottomLeftandCenter
  (bind _gridtilecount (Variables|Default|GetGridTileCount))
  (switch Utilities|FlowControl|Switch|SwitchonE_GridShape (Variables|Default|GetGridShape)
    (:NewEnumerator1
      (LocalVariables|SetC (CallFunction|SnapVectortoVector (Variables|Default|GetGridCenterLocation) (Variables|Default|GetGridTileSize)))
      (return (LocalVariables|GetC) (- (LocalVariables|GetC) (Math|Conversions|ToVector(Vector2D) (* (/ (- (Math|Conversions|ToVector2D(IntPoint) (Variables|Default|GetGridTileCount)) (Math|Vector2D|MakeVector2D (Math|Float|SelectFloat 0.0 1.0 (CallFunction|IsIntEven (.x _gridtilecount))) (Math|Float|SelectFloat 0.0 1.0 (CallFunction|IsIntEven (.y _gridtilecount))))) 2.0) (Math|Conversions|ToVector2D(Vector) (Variables|Default|GetGridTileSize)))))))
    (:NewEnumerator2
      (LocalVariables|SetC (CallFunction|SnapVectortoVector (Variables|Default|GetGridCenterLocation) (* (Variables|Default|GetGridTileSize) "1.500000,1.000000,1.000000")))
      (return (LocalVariables|GetC) (- (LocalVariables|GetC) (CallFunction|SnapVectortoVector (Math|Conversions|ToVector(Vector2D) (* (/ "" (Math|Conversions|ToVector2D(IntPoint) (Variables|Default|GetGridTileCount))) (Math|Conversions|ToVector2D(Vector) (Variables|Default|GetGridTileSize)))) (* (Variables|Default|GetGridTileSize) "1.500000,1.000000,1.000000")))))
    (:NewEnumerator3
      (LocalVariables|SetC (CallFunction|SnapVectortoVector (Variables|Default|GetGridCenterLocation) (* (Variables|Default|GetGridTileSize) "2.000000,1.000000,1.000000")))
      (return (LocalVariables|GetC) (- (LocalVariables|GetC) (CallFunction|SnapVectortoVector (Math|Conversions|ToVector(Vector2D) (* (/ (- (Math|Conversions|ToVector2D(IntPoint) (Variables|Default|GetGridTileCount)) (Math|Vector2D|MakeVector2D 1.0 1.0)) "(X=2.000000,Y=4.000000)") (Math|Conversions|ToVector2D(Vector) (Variables|Default|GetGridTileSize)))) (* (Variables|Default|GetGridTileSize) "2.000000,1.000000,1.000000")))))))

(fn GetTileRotationfromGridIndex
  (params (Grid%20Index :type Int%20Point%20Structure))
  (bind _gridtilecount (Variables|Default|GetGridTileCount))
  (if (Utilities|Enum|Equal(Enum) (Variables|Default|GetGridShape) "NewEnumerator3")
    (return (Math|Rotator|MakeRotator 0.0 0.0 (+ (Math|Float|SelectFloat 1.8e+02 0.0 (CallFunction|IsIntEven (.x _gridtilecount))) (Math|Float|SelectFloat 1.8e+02 0.0 (CallFunction|IsIntEven (.y _gridtilecount))))))
    (else
      (return "0, 0, 0"))))

(fn GetTileLocationfromGridIndex
  (params (InputPin :type Int%20Point%20Structure))
  (return (+ (Variables|Default|GetGridBottomLeftCornerLocation) (* (Variables|Default|GetGridTileSize) (Math|Conversions|ToVector(Vector2D) (* (Math|Conversions|ToVector2D(IntPoint) InputPin) (Utilities|Select :Index (Variables|Default|GetGridShape) :NewEnumerator0 "" :NewEnumerator1 "(X=1.000000,Y=1.000000)" :NewEnumerator2 "(X=0.750000,Y=0.500000)" :NewEnumerator3 "(X=1.000000,Y=0.500000)")))))))