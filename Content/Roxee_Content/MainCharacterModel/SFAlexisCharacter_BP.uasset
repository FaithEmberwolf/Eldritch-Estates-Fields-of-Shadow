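; Alexis main character Blueprint that manages first-person mesh visibility, an intro camera fade and interaction animation.
; Tick repeatedly applies a first-person component hide to the mesh.
; BeginPlay starts the widget camera fade and binds to the interaction manager's OnInteracted event.
; The interaction handler plays a right-arm pickup overlay montage when interaction is allowed and the target's primary method is not the one excluded type.
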(event Custom|CreateIntroWidgets
  (|CreateIntroWidgetsFunctionality))

(event EventTick
  (params (DeltaSeconds :type Float%20%28single-precision%29))
  (|SetCharacterVisiblity))

(event EventBeginPlay
  (|BeginPlay))

(fn ConstructionScript)

(event Custom|OnInteractedInput
  (params (TargetInteractionData :type Interactable%20Data%20S%20Structure))
  (bind _interactionmanager (CallFunction|GetSFInteractionManager(Controller)))
  (if (and (Variables|/Game/StoryFramework/Core/Blueprints/Components/Core/SFInteractionManager_AC.SFInteractionManager_AC_C|GetCanInteract _interactionmanager) (Utilities|Enum|NotEqual(Enum) (.PrimaryInteractionMethod (Utilities|Struct|BreakInteractionMethods_S (.interactionmethods (Variables|/Game/StoryFramework/Core/Blueprints/Components/Core/SFInteractionManager_AC.SFInteractionManager_AC_C|GetTargetInteractionActorData _interactionmanager)))) "NewEnumerator4"))
    (Animation|PlayAnimMontage "/Game/StoryFramework/Core/Example/Character/CharacterMeshes/Mannequins/Animations/Manny/MM_RightArmPickup_Overlay_Montage.MM_RightArmPickup_Overlay_Montage" 1.0 "None")))