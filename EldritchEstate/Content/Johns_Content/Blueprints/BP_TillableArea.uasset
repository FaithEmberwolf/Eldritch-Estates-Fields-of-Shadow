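; BP_TillableArea defines a rectangular tillable area intended to be divided into plots.
; The construction script sizes the flat TillableBox from Width and Height.
; It then runs a nested loop over that area in PlotSize steps, but the loop body is empty, so no plots are created yet.
; The event graph holds only disabled default events, so the asset has no runtime logic.
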(event EventBeginPlay)

(event Collision|EventActorBeginOverlap
  (params (OtherActor :type Actor%20Object%20Reference)))

(event EventTick
  (params (DeltaSeconds :type Float%20%28single-precision%29)))

(fn ConstructionScript
  ;[1 1 1] Set the tillable box size on start
  (Components|Box|SetBoxExtent (Variables|Default|GetTillableBox) (Math|Vector|MakeVector (/ (Variables|Default|GetWidth) 2.0) (/ (Variables|Default|GetHeight) 2.0) 1.0) true)
  ;[1 1 1] 2D For Loop (I think) to grid the area for plots
  (for _index (range 0 (Math|Float|Truncate (/ (Variables|Default|GetWidth) (Variables|Default|GetPlotSize))))
    (for _index_2 (range 0 (Math|Float|Truncate (/ (Variables|Default|GetHeight) (Variables|Default|GetPlotSize))))
      _)))