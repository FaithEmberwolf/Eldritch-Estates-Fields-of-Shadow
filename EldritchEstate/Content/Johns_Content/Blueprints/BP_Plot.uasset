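; BP_Plot is a farm plot that advances a plant through growth stages.
; On BeginPlay a looping five-second timer fires GrowingStage, which increments the plant state enum until it reaches its cap and prints each new stage to screen.
; A watered check exists in the graph but is not connected, so growth does not depend on watering.
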(event Custom|Growing%20Stage
  (if (not (>= (Math|Conversions|ToInteger(Byte) (Variables|Default|GetState)) 3))
    (bind _result (Math|Integer|IncrementInt (Math|Conversions|ToInteger(Byte) (Variables|Default|GetState)))
      (:%20%20
        ;[1 1 1] Change State
        (bind _output_get (Variables|Default|SetState (Utilities|Enum|ByteToEnumE_PlantState (Math|Conversions|ToByte(Integer) _result))))
        (Development|PrintString (Utilities|String|EnumtoString _output_get) true true "(R=0.000000,G=0.660000,B=1.000000,A=1.000000)" 2.0 "Plant")))))

(event EventBeginPlay
  (Utilities|Time|SetTimerbyEvent (delegate Custom|Growing%20Stage) 5.0 true))

(fn ConstructionScript)