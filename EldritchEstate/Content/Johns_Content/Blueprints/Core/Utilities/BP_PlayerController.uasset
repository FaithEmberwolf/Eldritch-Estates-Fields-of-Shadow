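; BP_PlayerController is a player controller built on SF framework components, with leftover farming prototype logic.
; BeginPlay applies the SFGameplay input mapping and loads SF components, Tick calls their getter without using the result, and the Inventory input opens the HUD's player menu.
; Disconnected chains hold HUD creation, cursor tracing to BP_Plot, tilling, watering, planting, harvesting and an interaction sphere trace; none of them run.
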(event EventBeginPlay
  (CallFunction|UpdateInputMappingContext "/Game/StoryFramwork/Content/StoryFramework/Core/Blueprints/ExampleInput/SFGameplay_IMC.SFGameplay_IMC" true)
  (CallFunction|LoadSFComponents(IntoMemory)))

(event EventTick
  (params (DeltaSeconds :type Float%20%28single-precision%29))
  (CallFunction|GetSFComponents))

(event Input|ActionEvents|InputActionInventory
  (params (Key :type Key%20Structure))
  ;[1 1 1] Virginia's inventory controls
  (:Pressed
    (Default|DisplayPlayerMenu (Variables|Default|GetHUD))))

(event Input|MouseEvents|LeftMouseButton
  (params (Key :type Key%20Structure))
  ;[1 1 1] If watering can Equiped
)

(event Input|KeyboardEvents|F
  (params (Key :type Key%20Structure))
  ;[1 1 1] Player Input
)

(event Input|MouseEvents|RightMouseButton
  (params (Key :type Key%20Structure))
  ;[1 1 1] If watering can Equiped
)

(fn ConstructionScript)

(fn GetSFComponents
  (return (Variables|Default|GetSFInteractionManager_AC) (Variables|Default|GetSFInventoryManager_AC) (Variables|Default|GetSFSequenceManager_AC) (Variables|Default|GetSFSaveManager_AC)))