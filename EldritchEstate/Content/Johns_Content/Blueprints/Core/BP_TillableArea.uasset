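; BP_TillableArea is an unfinished Blueprint for a tillable farming plot area.
; Its construction script sizes TillableBox from Width and Height, then runs nested grid loops that divide by zero and only clear RowArray.
; Nodes that would fill RowArray and PlotsArray with plant structs are disconnected.
; Tick loops over RowArray checking IsTilled but takes no action, and the helper function is an empty stub.
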(event EventTick
  (params (DeltaSeconds :type Float%20%28single-precision%29))
  (for _array_element (Variables|Default|GetRowArray)
    (if (Variables|Default|GetIsTilled?)
      _)))

(fn ConstructionScript
  (Components|Box|SetBoxExtent (Variables|Default|GetTillableBox) (Math|Vector|MakeVector (/ (Variables|Default|GetWidth) 2.0) (/ (Variables|Default|GetHeight) 2.0) 1.0) false)
  (for _index (range 0 (Math|Float|Truncate (/ (Variables|Default|GetWidth) 0.0)))
    (Utilities|Array|Clear (Variables|Default|GetRowArray))
    (for _index_2 (range 0 (Math|Float|Truncate (/ (Variables|Default|GetHeight) 0.0)))
      _)))

(fn NewFunction)