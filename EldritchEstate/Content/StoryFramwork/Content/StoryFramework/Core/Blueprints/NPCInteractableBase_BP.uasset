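; NPCInteractableBase_BP is the StoryFramework base Blueprint for NPCs that hold conversations when interacted with.
; BeginPlay initializes its interaction widget component, and Interactwith starts a conversation by passing itself and its dialogue sets to NPCManagerAC.
; Reply selections and end-of-reply input are forwarded to that manager to advance or stop the dialogue.
; The construction script sets the skeletal mesh's animation and offsets the HeadLocation component.
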(event Custom|InputReply
  (params (ReplyOption :type Text))
  ;[0.04314 0.04314 0.05098] Systems (Root)
  (Default|InputReply (Variables|Default|GetNPCManager_AC) ReplyOption))

(event Custom|InputEndReplies
  ;[0.04314 0.04314 0.05098] Systems (Root)
  (Default|StopConversation (Variables|Default|GetNPCManager_AC) false))

(event EventBeginPlay
  ;[0.04314 0.04314 0.05098] Systems (Root)
  (Default|UpdateInitialization (Variables|Default|GetSFInteractionWidget_SC)))

(event EventInteractwith
  (params (DataString :type String))
  ;[0.04314 0.04314 0.05098] Systems (Root)
  (CallFunction|StartConversation))

(fn ConstructionScript
  (Variables|/Script/Engine.SkeletalMeshComponent|SetAnimationData (Variables|Default|GetSkeletalMesh) (Utilities|Struct|MakeSingleAnimationPlayData (Variables|Default|GetAnimToPlay) true true 0.0))
  (Transformation|AddRelativeLocation (Variables|Default|GetHeadLocation) (Variables|Default|GetHeadLocationOffset) false false))

(fn StartConversation
  (Default|InitializeConversation (Variables|Default|GetNPCManager_AC) self (Variables|NPC|GetDialougeSets)))

(fn GetInteractionData
  (return ""))