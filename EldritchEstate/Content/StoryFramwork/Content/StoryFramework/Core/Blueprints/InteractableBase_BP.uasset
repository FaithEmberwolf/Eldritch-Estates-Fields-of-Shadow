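; Base Blueprint for Story Framework interactables, with a static mesh, a collision sphere and an interaction widget component.
; Construction runs UpdateCosmetics, which applies the object mesh and reinitializes the widget, then sets the sphere to a custom radius.
; Interactwith and LoadFromDataString, the Story Framework SaveGame hook, are empty events.
; UpdateInteractionData calls SetInteractionData, whose body is empty apart from unconnected refresh nodes.
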(event Custom|UpdateCosmetics
  (|UpdateCosmeticsLogic))

(event Custom|LoadFromDataString
  (params (DataString :type String)))

(event EventInteractwith
  (params (DataString :type String)))

(event EventUpdateInteractionData
  (params (InteractionData :type %20Structure))
  (|SetInteractionData InteractionData))

(fn ConstructionScript
  (CallFunction|UpdateCosmetics)
  (Components|Sphere|SetSphereRadius (Variables|Default|GetSphere) (Variables|Default|GetCustomCollisionRadius) true))