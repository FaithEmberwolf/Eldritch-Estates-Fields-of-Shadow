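; Blueprint function library of global gameplay helpers for the StoryFramework plugin, covering components, input, UI, camera, saving and dialog.
; Getters fetch interaction, inventory, sequence and save managers from player controller 0 through a message call, and other helpers build on them.
; Utilities toggle custom-depth outlines, swap Enhanced Input contexts, toggle a pause widget, record actor changes for saving, and check whether NPC dialog allows player movement.
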(fn OutlineActor(PostProcess)
  (params (Actor :type Actor%20Object%20Reference) (Remove :type Boolean))
  (bind _returnvalue (Actor|GetComponentsByClass Actor "/Script/Engine.SkeletalMeshComponent"))
  (bind _returnvalue_2 (Actor|GetComponentsByClass Actor "/Script/Engine.StaticMeshComponent"))
  (bind _returnvalue_3 (not Remove))
  (Utilities|IsValid Actor
    (:Is%20Valid
      (if (>= (Utilities|Array|LastIndex _returnvalue_2) 0)
        (for _array_element _returnvalue_2
          (Rendering|SetRenderCustomDepth _array_element _returnvalue_3)))
      (if (>= (Utilities|Array|LastIndex _returnvalue) 0)
        (for _array_element_2 _returnvalue
          (Rendering|SetRenderCustomDepth _array_element_2 _returnvalue_3))))))

(fn UpdateInputMappingContext
  (params (NewMappingContext :type Input%20Mapping%20Context%20Object%20Reference) (UpdateInteractionVariable :type Boolean))
  (bind _interactionmanager (ControllerInterface|GetSFInteractionManager(Controller)))
  (bind _returnvalue (Game|GetPlayerController 0))
  (bind _returnvalue_2 (PlayerController|LocalPlayerSubsystems|GetEnhancedInputLocalPlayerSubsystem _returnvalue))
  (Class|EnhancedInputSubsystemInterface|ClearAllMappings _returnvalue_2)
  (Input|AddMappingContext _returnvalue_2 NewMappingContext 0 (Utilities|Struct|MakeModifyContextOptions true false false))
  (if UpdateInteractionVariable
    (Utilities|IsValid _interactionmanager
      (:Is%20Valid
        (Variables|/Game/StoryFramwork/Content/StoryFramework/Core/Blueprints/Components/Core/SFInteractionManager_AC.SFInteractionManager_AC_C|SetCurrentInputMappingContext _interactionmanager NewMappingContext)))))

(fn GetSFSoundSettingsDataTable
  (bind _returnvalue (Utilities|GetDataTableRow "/Game/StoryFramwork/Content/StoryFramework/Core/Blueprints/DataTables/SFSoundSettings_DT.SFSoundSettings_DT" "Editable")
    (:then
      (return _returnvalue))))

(fn GetSFInteractionManager(Controller)
  (bind _interactionmanager (Class|SFPlayerControllerDataBPI|GetSFComponents(Message) (Game|GetPlayerController 0)))
  (return _interactionmanager))

(fn GetSFInventoryManager(Controller)
  (bind _inventorymanager (Class|SFPlayerControllerDataBPI|GetSFComponents(Message) (Game|GetPlayerController 0)))
  (return _inventorymanager))

(fn GetSFSequenceManager(Controller)
  (bind _sequencemanager (Class|SFPlayerControllerDataBPI|GetSFComponents(Message) (Game|GetPlayerController 0)))
  (return _sequencemanager))

(fn GetSFSaveManager(Controller)
  (bind _savemanager (Class|SFPlayerControllerDataBPI|GetSFComponents(Message) (Game|GetPlayerController 0)))
  (return _savemanager))

(fn SimpleFirstPersonComponentHide
  (params (Target :type Scene%20Component%20Object%20Reference))
  (bind _currentcamerapreset (Class|SFPlayerCameraManagerBPI|GetSFCameraData(Message) (Game|GetPlayerCameraManager 0)))
  (Rendering|SetVisibility Target (select (Default|IsCurrentSequencePlaying (ControllerInterface|GetSFSequenceManager(Controller))) true (Utilities|Select :Index _currentcamerapreset :Option%200 false :Option%201 false :Option%202 false)) false))

(fn DestroyActor(SaveGame)
  (params (Target :type Actor%20Object%20Reference))
  (Utilities|Array|Add 0 (Utilities|GetObjectName Target))
  (Actor|DestroyActor Target))

(fn SaveSpawnedActor(SaveGame)
  (params (Target :type Actor%20Object%20Reference%20%28by%20ref%29) (Interactable%20Data :type Interactable%20Data%20S%20Structure) (StaticMeshActor :type Static%20Mesh%20Object%20Reference))
  (Utilities|Array|Add :TargetArray (Variables|/Game/StoryFramwork/Content/StoryFramework/SaveGame/Blueprints/Components/SFSaveManager_AC.SFSaveManager_AC_C|GetSpawnedActors (ControllerInterface|GetSFSaveManager(Controller)))))

(fn TogglePauseGame(Widget)
  (params (PauseWidgetClass :type User%20Widget%20Class%20Reference) (UseWidgetNavInputMapping :type Boolean))
  (bind _returnvalue (Game|GetPlayerController 0))
  (bind _returnvalue_2 (Game|GetPlayerController 0))
  (LocalVariables|SetTargetUseWidgetNav UseWidgetNavInputMapping)
  (bind _foundwidgets (Widget|GetAllWidgetsOfClass 0 PauseWidgetClass))
  (Utilities|IsValid (Utilities|Array|Get(acopy) _foundwidgets)
    (:Is%20Valid
      (Widget|RemovefromParent (Utilities|Array|Get(acopy) _foundwidgets))
      (Game|SetGamePaused 0 false)
      (Variables|/Script/Engine.PlayerController|SetbShowMouseCursor _returnvalue_2 false)
      (Input|SetInputModeGameOnly _returnvalue_2 true)
      (if (LocalVariables|GetTargetUseWidgetNav)
        (CallFunction|UpdateInputMappingContext (Variables|Default|GetCurrentInputMappingContext (ControllerInterface|GetSFInteractionManager(Controller))) true)))
    (:Is%20Not%20Valid
      (bind _returnvalue_3 (UserInterface|CreateWidget PauseWidgetClass))
      (UserInterface|Viewport|AddtoViewport _returnvalue_3 0)
      (Game|SetGamePaused 0 true)
      (Variables|/Script/Engine.PlayerController|SetbShowMouseCursor _returnvalue true)
      (Input|SetInputModeGameandUI _returnvalue _returnvalue_3 "DoNotLock" false true)
      (if (LocalVariables|GetTargetUseWidgetNav)
        (CallFunction|UpdateInputMappingContext 0 false)))))

(fn UpdateInteractActors(SaveGame)
  (params (InteractActor :type %20Object%20Reference) (DataString :type String))
  (bind _savemanager (ControllerInterface|GetSFSaveManager(Controller)))
  (LocalVariables|SetTargetInteractActor 0 InteractActor)
  (LocalVariables|SetTargetInteractDataString DataString)
  (bind _keys (Utilities|Map|Keys (Variables|Default|GetInteractActors _savemanager)))
  (for _array_element _keys
    (Utilities|Array|Add (LocalVariables|GetFindInteractActorNames) _array_element))
  (Utilities|Map|Add (Variables|Default|GetInteractActors _savemanager) (Utilities|GetObjectName (.TargetInteractActor (LocalVariables|GetTargetInteractActor))) (LocalVariables|GetTargetInteractDataString)))

(fn LoadSystemInfo(SaveGame)
  (bind _returnvalue (SaveGame|LoadGamefromSlot "SFSaveSlot"))
  (bind _assfsave_game_bp (Utilities|Casting|CastToSFSaveGame_BP _returnvalue))
  (return (Variables|/Game/StoryFramwork/Content/StoryFramework/SaveGame/SFSaveGame_BP.SFSaveGame_BP_C|GetSystemData _assfsave_game_bp)))

(fn FindMenuButtoninMap(Widget)
  (params (NamedWidgetsMap :type Map%20of%20Names%20to%20Objects) (WidgetNavigationData :type Widget%20Navigation%20Data%20Structure%20%28by%20ref%29))
  (bind _widgettofocus (Utilities|Struct|BreakWidgetNavigationData WidgetNavigationData))
  (bind (_value _returnvalue) (Utilities|Map|Find NamedWidgetsMap _widgettofocus))
  (bind (_bsuccess _asmenu_button_w) (Utilities|Casting|CastTo _value))
  (if _returnvalue
    (if _bsuccess
      (Utilities|IsValid _asmenu_button_w
        (:Is%20Valid
          (CallFunction|CustomHoverButton _asmenu_button_w false))
        (:Is%20Not%20Valid
          _))
      (return _asmenu_button_w))))

(fn GetPauseMenuWidget(Reference)
  (bind _foundwidgets (Widget|GetAllWidgetsOfClass 0 0))
  (if (Utilities|Array|IsNotEmpty _foundwidgets)
    (return 0)
    (else
      (return 0))))

(fn GetSFCameraSettings(CameraManager)
  (bind _camerasettings (Class|Object|GetSFCameraData(Message) (Game|GetPlayerCameraManager 0)))
  (return _camerasettings))

(fn ResetSFCameraStates(CameraManager)
  (bind _sfcameramanagerref (Class|Object|GetSFCameraManager(Message) (Game|GetPlayerCameraManager 0)))
  (CallFunction|ResetStates _sfcameramanagerref))

(fn LoadSFComponents(IntoMemory)
  (CallFunction|LoadSelf (ControllerInterface|GetSFInteractionManager(Controller)))
  (CallFunction|LoadSelf (ControllerInterface|GetSFInventoryManager(Controller))))

(fn SFMovementCondition(DialogManager)
  (bind _interactionmanager (ControllerInterface|GetSFInteractionManager(Controller)))
  (if (and (Variables|Default|GetIsInDialogWithNPC _interactionmanager) (Utilities|IsValid (Variables|Default|GetTargetNPCActor _interactionmanager)))
    (return (Utilities|Struct|Break (Variables|Default|GetCurrentDialogSet (Variables|Default|GetNPCManager_AC (Variables|Default|GetTargetNPCActor _interactionmanager)))))
    (else
      (return true))))