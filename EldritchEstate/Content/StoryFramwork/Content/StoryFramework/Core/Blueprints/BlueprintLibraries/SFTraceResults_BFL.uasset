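; Blueprint function library in StoryFramework that exposes single-field getters for trace hit results.
; Each function takes a Hit Result and returns one member, such as blocking state, location, normals, hit actor or component, bone, or trace endpoints.
; It acts as a shortcut to avoid breaking the full struct, with no extra logic or validation.
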(fn GetBlockingHit
  (params (Hit%20Result :type Hit%20Result%20Structure))
  (return (.bBlockingHit (Collision|BreakHitResult Hit%20Result))))

(fn GetInitialOverlap
  (params (Hit%20Result :type Hit%20Result%20Structure))
  (return (.bInitialOverlap (Collision|BreakHitResult Hit%20Result))))

(fn GetTime
  (params (Hit%20Result :type Hit%20Result%20Structure))
  (return (.Time (Collision|BreakHitResult Hit%20Result))))

(fn GetDistance
  (params (Hit%20Result :type Hit%20Result%20Structure))
  (return (.Distance (Collision|BreakHitResult Hit%20Result))))

(fn GetLocation
  (params (Hit%20Result :type Hit%20Result%20Structure))
  (return (.Location (Collision|BreakHitResult Hit%20Result))))

(fn GetImpactPoint
  (params (Hit%20Result :type Hit%20Result%20Structure))
  (return (.ImpactPoint (Collision|BreakHitResult Hit%20Result))))

(fn GetNormal
  (params (Hit%20Result :type Hit%20Result%20Structure))
  (return (.Normal (Collision|BreakHitResult Hit%20Result))))

(fn GetImpactNormal
  (params (Hit%20Result :type Hit%20Result%20Structure))
  (return (.ImpactNormal (Collision|BreakHitResult Hit%20Result))))

(fn GetPhysMat
  (params (Hit%20Result :type Hit%20Result%20Structure))
  (return (.PhysMat (Collision|BreakHitResult Hit%20Result))))

(fn GetHitActor
  (params (Hit%20Result :type Hit%20Result%20Structure))
  (return (.HitActor (Collision|BreakHitResult Hit%20Result))))

(fn GetHitComponent
  (params (Hit%20Result :type Hit%20Result%20Structure))
  (return (.HitComponent (Collision|BreakHitResult Hit%20Result))))

(fn GetHitBoneName
  (params (Hit%20Result :type Hit%20Result%20Structure))
  (return (.HitBoneName (Collision|BreakHitResult Hit%20Result))))

(fn GetHitItem
  (params (Hit%20Result :type Hit%20Result%20Structure))
  (return (.HitItem (Collision|BreakHitResult Hit%20Result))))

(fn GetFaceIndex
  (params (Hit%20Result :type Hit%20Result%20Structure))
  (return (.FaceIndex (Collision|BreakHitResult Hit%20Result))))

(fn GetTraceStart
  (params (Hit%20Result :type Hit%20Result%20Structure))
  (return (.TraceStart (Collision|BreakHitResult Hit%20Result))))

(fn GetTraceEnd
  (params (Hit%20Result :type Hit%20Result%20Structure))
  (return (.TraceEnd (Collision|BreakHitResult Hit%20Result))))