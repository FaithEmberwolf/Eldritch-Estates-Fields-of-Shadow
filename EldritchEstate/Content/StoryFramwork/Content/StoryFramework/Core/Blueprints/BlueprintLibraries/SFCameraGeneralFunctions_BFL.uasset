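; Blueprint function library of StoryFramework camera helpers that act on player 0's camera manager.
; It attaches or detaches components, clamps pitch, reads gamepad use and camera states, and fades the view directly or through a fade widget.
; Field of view and distance setters switch on the current camera preset, rebuilding third- or first-person settings and sending them back by message.
; A small utility converts seconds into a play rate.
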(fn GetPlayRateLengthinSeconds
  (params (Length%28InSec%29 :type Float%20%28double-precision%29))
  (return (/ 1.0 Length%28InSec%29)))

(fn AttachComponenttoSFCamera
  (params (Target :type Scene%20Component%20Object%20Reference))
  (bind _returnvalue (Game|GetPlayerCameraManager 0))
  (bind _output_get (LocalVariables|SetTargetComponent Target))
  (LocalVariables|SetLensCameraManager _returnvalue)
  (Transformation|AttachComponentToComponent _output_get (Variables|/Script/Engine.PlayerCameraManager|GetTransformComponent _returnvalue) "None" "KeepRelative" "SnapToTarget" "KeepRelative" true)
  (bind _sfcameramanagerref (Class|Object|GetSFCameraManager(Message) (LocalVariables|GetLensCameraManager)))
  (Transformation|SetWorldRotation (LocalVariables|GetTargetComponent) (Camera|GetCameraRotation (LocalVariables|GetLensCameraManager)) false false))

(fn DetachComponentfromSFCamera
  (params (Target :type Scene%20Component%20Object%20Reference))
  (bind _output_get (LocalVariables|SetTargetComponent Target))
  (Transformation|DetachFromComponent _output_get "KeepRelative" "KeepRelative" "KeepRelative" true))

(fn SetCameraFieldOfView
  (params (FieldOfView :type Float%20%28double-precision%29))
  (LocalVariables|SetTargetFieldOfView FieldOfView)
  (bind _output_get (LocalVariables|SetPlayerCameraManager (Game|GetPlayerCameraManager 0)))
  (bind _sfcameramanagerref (Class|Object|GetSFCameraManager(Message) _output_get))
  (switch Utilities|FlowControl|Switch|Switchon (Variables|Default|GetCurrentCameraPreset _sfcameramanagerref)
    (:NewEnumerator3
      (Class|Object|SetCameraSettings(Message) (LocalVariables|GetPlayerCameraManager) (|ThirdPersonSettings _sfcameramanagerref (LocalVariables|GetTargetFieldOfView))))
    (:NewEnumerator4
      (Class|Object|SetCameraSettings(Message) (LocalVariables|GetPlayerCameraManager) (|FirstPersonSettings _sfcameramanagerref (LocalVariables|GetTargetFieldOfView))))))

(fn SetCameraDistance
  (params (CameraDistance :type Float%20%28double-precision%29))
  (LocalVariables|SetDistance CameraDistance)
  (bind _output_get (LocalVariables|SetPlayerCameraManager (Game|GetPlayerCameraManager 0)))
  (bind _sfcameramanagerref (Class|Object|GetSFCameraManager(Message) _output_get))
  (switch Utilities|FlowControl|Switch|Switchon (Variables|Default|GetCurrentCameraPreset _sfcameramanagerref)
    (:NewEnumerator3
      (Class|Object|SetCameraSettings(Message) (LocalVariables|GetPlayerCameraManager) (|ThirdPersonSettings _sfcameramanagerref (LocalVariables|GetDistance))))
    (:NewEnumerator4
      (Class|Object|SetCameraSettings(Message) (LocalVariables|GetPlayerCameraManager) (|FirstPersonSettings _sfcameramanagerref (LocalVariables|GetDistance))))))

(fn IsUsingGamepad
  (bind _sfcameramanagerref (Class|Object|GetSFCameraManager(Message) (Game|GetPlayerCameraManager 0)))
  (return (Variables|Default|GetIsUsingGamepad _sfcameramanagerref)))

(fn GetSFCameraStates
  (bind _sfcameramanagerref (Class|Object|GetSFCameraManager(Message) (Game|GetPlayerCameraManager 0)))
  (return (Variables|Default|GetCameraStates _sfcameramanagerref)))

(fn SetCameraPitchClamps
  (params (View%20Pitch%20Min :type Float%20%28single-precision%29) (View%20Pitch%20Max :type Float%20%28single-precision%29))
  (bind _sfcameramanagerref (Class|Object|GetSFCameraManager(Message) (Game|GetPlayerCameraManager 0)))
  (CallFunction|ClampCameraPitch _sfcameramanagerref View%20Pitch%20Min View%20Pitch%20Max))

(fn FadeCamera
  (params (FromAlpha :type Float%20%28single-precision%29) (ToAlpha :type Float%20%28single-precision%29) (Duration :type Float%20%28single-precision%29) (Color :type Linear%20Color%20Structure) (bShouldFadeAudio :type Boolean) (bHoldWhenFinished :type Boolean))
  (CameraFades|StartCameraFade (Game|GetPlayerCameraManager 0) FromAlpha ToAlpha Duration Color bShouldFadeAudio bHoldWhenFinished))

(fn WidgetFadeCamera
  (params (FadeDirection :type Integer) (FadeSpeed%20%28InSec%29 :type Float%20%28double-precision%29))
  (LocalVariables|SetFadeDirRef FadeDirection)
  (LocalVariables|SetFadeSpeedRef FadeSpeed%20%28InSec%29)
  (bind _foundwidgets (Widget|GetAllWidgetsOfClass 0 0))
  (Utilities|IsValid (Utilities|Array|Get(acopy) _foundwidgets)
    (:Is%20Valid
      (LocalVariables|SetWidgetFadeRef 0 0))
    (:Is%20Not%20Valid
      (bind _returnvalue (UserInterface|CreateWidget 0))
      (LocalVariables|SetWidgetFadeRef 0 _returnvalue)))
  (Variables|Default|SetFadeDirection (.WidgetFadeRef (LocalVariables|GetWidgetFadeRef)) (LocalVariables|GetFadeDirRef))
  (Variables|Default|SetFadeSpeed%28InSec%29 (.WidgetFadeRef (LocalVariables|GetWidgetFadeRef)) (LocalVariables|GetFadeSpeedRef))
  (CallFunction|StartFade (.WidgetFadeRef (LocalVariables|GetWidgetFadeRef)))
  (UserInterface|Viewport|AddtoViewport (.WidgetFadeRef (LocalVariables|GetWidgetFadeRef)) 2))